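; Player-controlled hover ship pawn, driven by physics forces and torques on Spacer from move, turn and boost input.
; Each tick, four downward sphere traces (front, back, left, right) align the ship to the ground and hold hover height, flagging flight when any misses.
; Hits cost health with an explosion, behind a delay-reset DoOnce; zero health reloads the level.
; A boost meter drains and refills, and HudState exposes stats for display.
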(event `self.Spacer.OnComponentHit`
  (params (OtherActor :type "Actor Object Reference") (OtherComp :type "PrimitiveComponent Object Reference") (NormalImpulse :type "Vector Structure") (Hit :type "HitResult Structure (by ref)"))
  (bind _returnvalue (`SceneComponent.K2_GetComponentLocation` (`self.Spacer`)))
  (`|ExecutionSequence`
    (:`then_0`
      (`/Engine/EditorBlueprintResources/StandardMacros.DoOnce` false :!label _label
        (:`Completed`
          ;[1 1 1] Comment
          (set `self.currentHealth` (- (`self.currentHealth`) 10.0))
          (bind _returnvalue_2 (`GameplayStatics.SpawnSoundAtLocation` "/Game/StarterContent/Audio/Explosion02.Explosion02" _returnvalue))
          (set `self.Audio` _returnvalue_2)
          (`GameplayStatics.SpawnEmitterAtLocation` "/Game/StarterContent/Particles/P_Explosion.P_Explosion" _returnvalue))))
    (:`then_1`
      (`KismetSystemLibrary.Delay` 1.0)
      (goto _label :!via `Reset`))))

(event `self.ReceiveTick`
  (params (DeltaSeconds :type "Float (single-precision)"))
  (bind _mindistance (`self.MinDistance`))
  (bind _averagedistance (`self.AverageDistance`))
  (bind _returnvalue (`SceneComponent.K2_GetComponentRotation` (`self.Spacer`)))
  (bind _returnvalue_2 (`SceneComponent.GetUpVector` (`self.Spacer`)))
  (bind _returnvalue_3 (* (* DeltaSeconds (`self.GetInputAxisValue`)) (`self.TurnSpeed`)))
  (bind _returnvalue_4 (+ (`KismetMathLibrary.MakeVector` (.z (`KismetMathLibrary.LessLess_VectorRotator` (- (`self.ShipRoll`) (`self.GroundRoll`)) _returnvalue))) (`KismetMathLibrary.MakeVector` 0.0 (.z (`KismetMathLibrary.LessLess_VectorRotator` (- (`self.ShipPitch`) (`self.GroundPitch`)) _returnvalue)))))
  (`|ExecutionSequence`
    (:`then_0`
      ;[1 1 1] Handle User Input
      (`PrimitiveComponent.AddForce` (`self.Spacer`) (* (* (* (`self.GetActorForwardVector`) (* (`self.GetInputAxisValue`) DeltaSeconds)) (+ (`self.MovementSpeed`) (* (`KismetMathLibrary.Conv_BoolToInt` (`self.isBoosting`)) (`self.Boost`)))) 10.0) "None" true)
      (`PrimitiveComponent.AddTorque` (`self.Spacer`) (* (`KismetMathLibrary.GreaterGreater_VectorRotator` (`KismetMathLibrary.MakeVector` (* _returnvalue_3 -0.4) 0.0 _returnvalue_3) (`self.K2_GetActorRotation`)) 10.0) "None" true))
    (:`then_1`
      ;[1 1 1] Check for Ground
      (bind (_location _distance _hit) (`self.LineTraceDown` (`self.FrontStart`)))
      (bind (_location_2 _distance_2 _hit_2) (`self.LineTraceDown` (`self.BackStart`)))
      (if (and _hit _hit_2 (stale _hit_3) (stale _hit_4)) :!label _label_2
        (set `self.isFlying` false)
        (set `self.GroundPitch` (- _location _location_2))
        (set `self.GroundRoll` (- (stale _location_3) (stale _location_4)))
        (set `self.AverageDistance` (/ (+ _distance _distance_2 (stale _distance_3) (stale _distance_4)) 4.0))
        (else
          (set `self.GroundPitch` (* (`self.GroundRoll`) -1.0))
          (set `self.GroundRoll` (* (`self.GroundRoll`) -1.0))
          (set `self.AverageDistance` (+ (`self.MaxDistance`) 1.0))
          (set `self.isFlying` true))))
    (:`then_2`
      (bind (_location_3 _distance_3 _hit_3) (`self.LineTraceDown` (`self.LeftStart`)))
      (bind (_location_4 _distance_4 _hit_4) (`self.LineTraceDown` (`self.RightStart`)))
      (goto _label_2))
    (:`then_3`
      ;[1 1 1] Orient to Ground
      (set `self.ShipPitch` (- (`SceneComponent.K2_GetComponentLocation` (`self.FrontStart`)) (`SceneComponent.K2_GetComponentLocation` (`self.BackStart`))))
      (set `self.ShipRoll` (- (`SceneComponent.K2_GetComponentLocation` (`self.LeftStart`)) (`SceneComponent.K2_GetComponentLocation` (`self.RightStart`))))
      (if (not (`self.isFlying`))
        _
        (else
          _))
      (`PrimitiveComponent.AddTorque` (`self.Spacer`) (* _returnvalue_4 5000.0) "None" false)
      (`PrimitiveComponent.SetPhysicsAngularVelocity` (`self.Spacer`) (`KismetMathLibrary.GreaterGreater_VectorRotator` _returnvalue_4 _returnvalue) false "None"))
    (:`then_4`
      ;[1 1 1] Ground Offset
      (if (> _averagedistance _mindistance)
        (`PrimitiveComponent.SetEnableGravity` (`self.Spacer`) (`self.isFlying`))
        (set `self.zAdd` (* (* _returnvalue_2 (- (`self.TargetDistance`) (`self.AverageDistance`))) 5000.0))
        (else
          (`SceneComponent.K2_AddWorldOffset` (`self.Spacer`) (* _returnvalue_2 (- _mindistance _averagedistance)) false true)))
      (`PrimitiveComponent.AddForce` (`self.Spacer`) (`self.zAdd`) "None" false))
    (:`then_5`
      (`self.Update Stats`))
    (:`then_6`
      (`self.dead`))))

(event `self.ReceiveBeginPlay`
  ;[1 1 1] Setting startStats
  (`self.setStartStats`))

(event `InputAction|Boost`
  (params (Key :type "Key Structure" :default "AnyKey"))
  (:`Pressed`
    (set `self.isBoosting` true))
  (:`Released`
    (set `self.isBoosting` false)))

(event `dead`
  ;[1 1 1] Reset level when currentHealth <= 0
  (if (<= (`self.currentHealth`) 0.0)
    (bind _returnvalue (`GameplayStatics.GetCurrentLevelName` true))
    (`GameplayStatics.OpenLevel` (`KismetStringLibrary.Conv_StringToName` _returnvalue))))

(event `Update Stats`
  (bind _movementspeed (`self.MovementSpeed`))
  ;[1 1 1] update Stats every frame
  (`|ExecutionSequence`
    (:`then_0`
      ;;[1 1 1] Drain Boostmeter when boosting
      (if (`self.isBoosting`)
        (set `self.currentBoost` (- (`self.currentBoost`) 1.0))
        (else
          ;;[1 1 1] Slowly filling boostmeter when not boosting
          (if (< (`self.currentBoost`) (`self.maxBoost`))
            (`KismetSystemLibrary.Delay` 0.5)
            (set `self.currentBoost` (+ (`self.currentBoost`) 10.0))))))
    (:`then_1`
      ;;[1 1 1] update visual current speed
      (if (`self.isBoosting`)
        (set `self.currentSpeed` (+ _movementspeed (`self.Boost`)))
        (else
          (set `self.currentSpeed` _movementspeed))))
    (:`then_2`
      ;;[1 1 1] turning off boostfunction when out of boost
      (if (<= (`self.currentBoost`) 0.0)
        (set `self.isBoosting` false)))))

(fn `hudState`
  (returns (currentHealth :type "Float (double-precision)") (maxHealth :type "Float (double-precision)") (currentBoost :type "Float (double-precision)") (maxBoost :type "Float (double-precision)") (currentspeed :type "Float (double-precision)") (maxSpeed :type "Float (double-precision)") (shipName :type Text) (currentExp :type Integer))
  (return (`self.currentHealth`) (`self.maxHealth`) (`self.currentBoost`) (`self.maxBoost`) (`self.currentSpeed`) (`self.maxSpeed`) (`self.shipName`) (`self.currentExp`)))

(fn `LineTraceDown`
  (params (Start :type "SceneComponent Object Reference"))
  (returns (Location :type "Vector Structure") (Distance :type "Float (double-precision)") (Hit :type Boolean))
  (bind _returnvalue (`SceneComponent.K2_GetComponentLocation` Start))
  (bind (_outhit _returnvalue_2) (`KismetSystemLibrary.SphereTraceSingleForObjects` _returnvalue (+ _returnvalue (* (`SceneComponent.GetForwardVector` Start) 2000.0)) 50.0 (`|MakeArray` "ObjectTypeQuery1" :!type "EObjectTypeQuery Enum")))
  (bind (_bblockinghit _binitialoverlap _time _location) (`GameplayStatics.BreakHitResult` _outhit))
  (return _location (`KismetMathLibrary.VSize` (- _returnvalue _location)) _returnvalue_2))

(fn `setStartStats`
  (`|ExecutionSequence`
    (:`then_0`
      (set `self.shipName` (`KismetTextLibrary.Conv_StringToText` (`KismetSystemLibrary.GetObjectName` (`self.Spacer`)))))
    (:`then_1`
      (set `self.currentHealth` (`self.maxHealth`)))
    (:`then_2`
      (set `self.maxBoost` 100.0))
    (:`then_3`
      (set `self.currentBoost` 0.0))
    (:`then_4`
      (set `self.currentExp` 0))))

(fn `UserConstructionScript`)